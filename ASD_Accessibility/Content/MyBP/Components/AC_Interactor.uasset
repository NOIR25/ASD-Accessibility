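; Interaction component that lets the player point at and tap world objects with a gamepad-driven mouse cursor.
; Stick input moves the cursor by a sensitivity multiplier, and a Visibility trace from the deprojected cursor finds actors implementing BPI_Interactions.
; Hovered actors receive LookAt, gated by a DoOnce that resets when the hit actor changes, while IA_Interact sends TapInteract.
; Both messages pass the player and fire matching OnLookAt and OnTapInteract calls.
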(event `self.ReceiveBeginPlay`
  (`self.FetchClasses`))

(event `EnhancedInput|/Game/MyBP/Input/IA_Interact`
  (params (ActionValue :type Boolean) (ElapsedSeconds :type "Float (double-precision)") (TriggeredSeconds :type "Float (double-precision)") (InputAction :type "InputAction Object Reference" :default "/Game/MyBP/Input/IA_Interact.IA_Interact"))
  ;[0 0 0] Checks for interactable objects on trace hit
  ; Calls Tap interact function
  (:`Started`
    (bind _outhit (`self.LineTraceFromMousePosition` 10000.0))
    (bind (_bblockinghit _binitialoverlap _time _distance _location _impactpoint _normal _impactnormal _physmat _hitactor) (`GameplayStatics.BreakHitResult` _outhit))
    (if (`KismetSystemLibrary.DoesImplementInterface` _hitactor "/Game/MyBP/Interfaces/BPI_Interactions.BPI_Interactions_C")
      (set `self.InteractingActor` _hitactor)
      (`/Engine/EditorBlueprintResources/StandardMacros.IsValid` (`self.My Player`)
        (:`Is Valid`
          (message `/Game/MyBP/Interfaces/BPI_Interactions.Tap Interact` (`self.InteractingActor`) (`self.My Player`))
          (`self.OnTapInteract`))))))

(event `EnhancedInput|/Game/MyBP/Input/IA_Cursor`
  (params (ActionValue :type "Vector2D Structure") (ElapsedSeconds :type "Float (double-precision)") (TriggeredSeconds :type "Float (double-precision)") (InputAction :type "InputAction Object Reference" :default "/Game/MyBP/Input/IA_Cursor.IA_Cursor"))
  ;[0 0 0] Sets Mouse Position through gamepad input.
  ; Checks Hit objects to see if they are interactable (UI / Haptics)
  (:`Triggered`
    (`self.SetMousePosition` ActionValue_X ActionValue_Y)
    (bind _outhit (`self.LineTraceFromMousePosition` 10000.0))
    (bind (_bblockinghit _binitialoverlap _time _distance _location _impactpoint _normal _impactnormal _physmat _hitactor) (`GameplayStatics.BreakHitResult` _outhit))
    (if (!= _hitactor (`self.HoveredActor`))
      (`self.CE_ResetLookAt`))
    (if (`KismetSystemLibrary.DoesImplementInterface` _hitactor "/Game/MyBP/Interfaces/BPI_Interactions.BPI_Interactions_C")
      (set `self.HoveredActor` _hitactor)
      (`/Engine/EditorBlueprintResources/StandardMacros.IsValid` (`self.My Player`)
        (:`Is Valid`
          (`/Engine/EditorBlueprintResources/StandardMacros.DoOnce` false :!label _label
            (:`Completed`
              (bind _hoveredactor (`self.HoveredActor`)
                (:`then`
                  (message `/Game/MyBP/Interfaces/BPI_Interactions.LookAt` _hoveredactor (`self.My Player`))
                  (`self.OnLookAt`))
                (:`else`))))))
      (else
        (set `self.HoveredActor` null)))))

(event `CE_ResetLookAt`
  ;[0 0 0] Sets Mouse Position through gamepad input.
  ; Checks Hit objects to see if they are interactable (UI / Haptics)
  (goto _label :!via `Reset`))

(fn `FetchClasses`
  (bind _myplayer (message `/Game/MyBP/Interfaces/BPI_ClassFetcher.GetMyPlayer` (`self.GetOwner`)))
  (set `self.My Player` _myplayer)
  (bind _mycontroller (`/Game/MyBP/BFL/BFL_ClassFetcher.GetPC`))
  (set `self.My Controller` _mycontroller))