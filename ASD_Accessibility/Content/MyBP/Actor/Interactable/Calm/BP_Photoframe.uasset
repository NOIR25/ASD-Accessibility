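; BP_Photoframe is an interactable photo frame that can start crooked and be straightened with a tap.
; The construction script sets the mesh and tints a dynamic material with a random palette colour.
; When IsMisaligned, BeginPlay applies random pitch and TapInteract runs a timeline easing the frame to zero rotation and a slight offset, though it leaves IsMisaligned true.
; Looking at the frame plays haptic feedback on the player controller.
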(event `self.ReceiveBeginPlay`
  (`self.FetchClasses`)
  (if (`self.isMisaligned`)
    (`self.ApplyRandomRotation` -10.0 10.0)))

(event `/Game/MyBP/Interfaces/BPI_Interactions.Tap Interact`
  (params (Interactor :type "Actor Object Reference"))
  (set `self.Interactor` Interactor)
  (if (`self.isMisaligned`)
    (bind (_direction _alpha) (`Timeline|LerpFrame` :!via `PlayFromStart`)
      (:`Update`
        (`SceneComponent.K2_SetRelativeRotation` (`self.Frame`) (`KismetMathLibrary.RLerp` (`SceneComponent.RelativeRotation` (`self.Frame`)) (struct) _alpha) false false)
        (`SceneComponent.K2_SetRelativeLocation` (`self.Frame`) (`KismetMathLibrary.VLerp` (`SceneComponent.RelativeLocation` (`self.Frame`)) (0.0 -2.0 0.0) _alpha) false false)
        (set `self.isMisaligned` true)))))

(event `/Game/MyBP/Interfaces/BPI_Interactions.LookAt`
  (params (interactor :type "/Game/MyBP/Actor/Player/BP_MyPlayer Object Reference"))
  (`PlayerController.K2_ClientPlayForceFeedback` (`self.My Controller`) (`self.LookAtHaptic`) "None" false false false))

(fn `ApplyRandomRotation`
  (params (Min :type "Float (double-precision)") (Max :type "Float (double-precision)"))
  (`SceneComponent.K2_SetRelativeRotation` (`self.Frame`) (`KismetMathLibrary.MakeRotator` 0.0 (`KismetMathLibrary.RandomFloatInRange` Min Max)) false false))

(fn `FetchClasses`
  (bind _mycontroller (`/Game/MyBP/BFL/BFL_ClassFetcher.GetPC`))
  (set `self.My Controller` _mycontroller))

(fn `UserConstructionScript`
  (bind _pallete1 (`self.Pallete1`))
  ;[0 0 0] Set Start Mesh
  (`StaticMeshComponent.SetStaticMesh` (`self.Frame`) (`self.FrameMesh`))
  (bind _returnvalue (`PrimitiveComponent.CreateDynamicMaterialInstance` (`self.Frame`) 0 "/Game/Meshes/Materials/MI_Base.MI_Base" "None"))
  (bind _output_get (set `self.DynamicMaterial` _returnvalue))
  (`MaterialInstanceDynamic.SetVectorParameterValue` _output_get "Colour" (`|GetArrayItem` _pallete1 (`KismetMathLibrary.RandomIntegerInRange` 0 (`KismetArrayLibrary.Array_LastIndex` _pallete1)))))