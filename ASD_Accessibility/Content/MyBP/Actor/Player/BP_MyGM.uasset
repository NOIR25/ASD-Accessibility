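; Game mode that tracks a daily login streak and the player's current mood.
; Game-instance load and first-login events drive it, with save data read and written asynchronously through the game instance.
; On load, elapsed time since last login selects error, restart, no change or increment, and sets countdown text; error and no-change handlers are empty stubs.
; Mood updates broadcast a dispatcher and print the new state.
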(event `self.ReceiveBeginPlay`
  (`self.FetchClasses`)
  (`self.BindToDispatchers`)
  (set `PlayerController.bShowMouseCursor` true (`self.My Controller`)))

(event `/Game/MyBP/Interfaces/BPI_UI.UpdateMood`
  (params (Mood :type "/Game/MyBP/Enums/E_Moods Enum" :default "NewEnumerator0"))
  (`self.OnMoodChanged` Mood)
  (bind _output_get (set `self.EMoods` Mood))
  (switch `/Game/MyBP/Enums/E_Moods` _output_get
    (:`NewEnumerator0`
      (`KismetSystemLibrary.PrintString` "You are calm"))
    (:`NewEnumerator5`
      (`KismetSystemLibrary.PrintString` "You are focused"))
    (:`NewEnumerator1`
      (`KismetSystemLibrary.PrintString` "You are over-stimulated"))
    (:`NewEnumerator2`
      (`KismetSystemLibrary.PrintString` "You are restless"))))

(event `On First Login`
  (bind _output_get (set `self.FirstLogin` (`KismetMathLibrary.Now`)))
  (set `self.LastLoggedIn` _output_get)
  (`self.Increase Streak`)
  (`/Game/MyBP/BFL/BFL_HelperFunctions.SaveGMData` true)
  (`KismetSystemLibrary.PrintString` "First Log in"))

(event `OnGameLoad`
  (`self.InitialiseSaveData`)
  (`self.CompareLoginDate`)
  (switch `int` (`self.CommandIndex`)
    (:`0`
      (`self.ErrorStreak`))
    (:`1`
      (`self.Restart Streak`))
    (:`2`
      (`self.NoStreak`))
    (:`3`
      (`self.Increase Streak`)))
  (set `self.LastLoggedIn` (`KismetMathLibrary.Now`))
  (`KismetSystemLibrary.PrintString` (`KismetStringLibrary.Conv_IntToString` (`self.CurrentStreak`)))
  (`/Game/MyBP/BFL/BFL_HelperFunctions.SaveGMData` true))

(event `SaveGMData`
  (params (Async :type Boolean))
  (bind _gmsave (`self.GetGMSave`))
  (message `/Game/MyBP/Interfaces/BPI_SaveGame.SaveGM` (`GameplayStatics.GetGameInstance`) _gmsave Async))

(fn `BindToDispatchers`
  (bind _mygi (`self.MyGI`)
    (:`then`
      (add `/Game/MyBP/Actor/Player/BP_GameInstance.OnGameLoaded` _mygi (`|CreateDelegate` :!event `OnGameLoad`))
      (add `self.OnFirstLogin` (`|CreateDelegate` :!event `On First Login`)))
    (:`else`)))

(fn `CompareLoginDate`
  (bind (_notyettime _errorfuture) (`self.Date Display` (* (- (`KismetMathLibrary.Now`) (+ (`self.LastLoggedIn`) (`KismetMathLibrary.MakeTimespan` 1))) (`KismetMathLibrary.SelectInt` -1 1 (< (`self.LoginDifference`) (`KismetMathLibrary.MakeTimespan` 1))))))
  ;[0.2865 0.1802 0.08213] Set the difference between Now and Last Login
  (set `self.LoginDifference` (- (`KismetMathLibrary.Now`) (`self.LastLoggedIn`)))
  ;[0.3646 0.2514 0.1295] was the last login less than than 0 days ago?
  (if (< (`self.LoginDifference`) (`KismetMathLibrary.MakeTimespan` 0))
    (set `self.TimeLeft` _errorfuture)
    (set `self.CommandIndex` 0)
    (else
      ;[0.3177 0.2172 0.1145] was the last login greater than 2 days ago?
      (if (> (`self.LoginDifference`) (`KismetMathLibrary.MakeTimespan` 2))
        (set `self.CommandIndex` 1)
        (else
          ;[0.3385 0.2179 0.08695] was the last login greater or equal than 1 day ago?
          (if (<= (`self.LoginDifference`) (`KismetMathLibrary.MakeTimespan` 1))
            (set `self.TimeLeft` _notyettime)
            (set `self.CommandIndex` 2)
            (else
              (set `self.TimeLeft` (`KismetStringLibrary.Concat_StrStr` "0" "Seconds" "Left"))
              (set `self.CommandIndex` 3))))))))

(fn `Date Display`
  (params (Time :type "Timespan Structure"))
  (returns (NotYetTime :type String) (ErrorFuture :type String))
  (bind (_days _hours _minutes _seconds) (`KismetMathLibrary.BreakTimespan` Time))
  (bind (_days_2 _hours_2 _minutes_2 _seconds_2) (`KismetMathLibrary.BreakTimespan` Time))
  (return (`KismetMathLibrary.SelectString` (`KismetStringLibrary.Concat_StrStr` "0" "Days " "23" "Hours " "59" "Minutes " "59" "Seconds ") (`KismetStringLibrary.Concat_StrStr` "0" "Days " (`KismetStringLibrary.Conv_IntToString` _hours_2) "Hours " (`KismetStringLibrary.Conv_IntToString` _minutes_2) "Minutes " (`KismetStringLibrary.Conv_IntToString` _seconds_2) "Seconds ") (== _days_2 1)) (`KismetStringLibrary.Concat_StrStr` (`KismetStringLibrary.Conv_IntToString` _days) "Days " (`KismetStringLibrary.Conv_IntToString` _hours) "Hours " (`KismetStringLibrary.Conv_IntToString` _minutes) "Minutes " (`KismetStringLibrary.Conv_IntToString` _seconds) "Seconds ")))

(fn `ErrorStreak`)

(fn `FetchClasses`
  (bind _mycontroller (`/Game/MyBP/BFL/BFL_ClassFetcher.GetPC`))
  (set `self.My Controller` _mycontroller)
  (bind _mygameinstance (`/Game/MyBP/BFL/BFL_ClassFetcher.GetGI`))
  (set `self.MyGI` _mygameinstance))

(fn `GetGMSave`
  (returns (GMSave :type "/Game/MyBP/Structs/S_SaveData Structure"))
  (return (make `/Game/MyBP/Structs/S_SaveData` (`self.FirstLogin`) (`self.LastLoggedIn`) (`self.CurrentStreak`))))

(fn `GetMyGI`
  (returns (MyGameInstance :type "/Game/MyBP/Actor/Player/BP_GameInstance Object Reference"))
  (return null))

(fn `GetMyGM`
  (returns (MyGamemode :type "/Game/MyBP/Actor/Player/BP_MyGM Object Reference"))
  (return self))

(fn `GetMyHUD`
  (returns (HUD :type "/Game/MyBP/UI/BP_HUD Object Reference"))
  (return null))

(fn `GetMyPC`
  (returns (MyController :type "/Game/MyBP/Actor/Player/BP_MyPC Object Reference"))
  (return null))

(fn `GetMyPlayer`
  (returns (MyPlayer :type "/Game/MyBP/Actor/Player/BP_MyPlayer Object Reference"))
  (return null))

(fn `Increase Streak`
  (set `self.CurrentStreak` (+ (`self.CurrentStreak`) 1)))

(fn `InitialiseSaveData`
  ;[0.4583 0.3333 0.1789] Fetches saved data if valid and sets this classes variables to our saved data
  (bind _savegamedata (message `/Game/MyBP/Interfaces/BPI_SaveGame.GetGameData` (`GameplayStatics.GetGameInstance`)))
  (`/Engine/EditorBlueprintResources/StandardMacros.IsValid` _savegamedata
    (:`Is Valid`
      (`self.UseGMSave` (`/Game/MyBP/SaveGame/BP_SaveGame.S_SaveGameData` _savegamedata)))))

(fn `NoStreak`)

(fn `Restart Streak`
  (set `self.CurrentStreak` 0))

(fn `UseGMSave`
  (params (GMSave :type "/Game/MyBP/Structs/S_SaveData Structure"))
  (set `self.FirstLogin` GMSave_PlayerFirstLogin_29_A3C230C64D00260A02D58198C4A46818)
  (set `self.LastLoggedIn` GMSave_PlayerLastLoggedIn_32_3FE3B13C41372408D03E1D8A6879FD17)
  (set `self.CurrentStreak` GMSave_CurrentStreak_37_A18A45FD4CD2E35CB37CBD87A97452DD))

(fn `UserConstructionScript`)