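; BP_MyPlayer is the player Blueprint, currently a skeleton for saving and restoring player data such as the current streak.
; BeginPlay caches the game instance through ClassFetcher.
; InitialiseSaveData, not called here, passes valid game-instance save data to UsePlayerSave, which is an empty stub.
; GetPlayerSave returns a zero streak, and of the GetMy accessors only GetMyPlayer returns a value, itself.
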(event `self.ReceiveBeginPlay`
  (`self.ClassFetcher`))

(fn `ClassFetcher`
  (bind _mygameinstance (`/Game/MyBP/BFL/BFL_ClassFetcher.GetGI`))
  (set `self.My Game Instance` _mygameinstance))

(fn `GetMyGI`
  (returns (MyGameInstance :type "/Game/MyBP/Actor/Player/BP_GameInstance Object Reference"))
  (return null))

(fn `GetMyGM`
  (returns (MyGamemode :type "/Game/MyBP/Actor/Player/BP_MyGM Object Reference"))
  (return null))

(fn `GetMyHUD`
  (returns (HUD :type "/Game/MyBP/UI/BP_HUD Object Reference"))
  (return null))

(fn `GetMyPC`
  (returns (MyController :type "/Game/MyBP/Actor/Player/BP_MyPC Object Reference"))
  (return null))

(fn `GetMyPlayer`
  (returns (MyPlayer :type "/Game/MyBP/Actor/Player/BP_MyPlayer Object Reference"))
  (return self))

(fn `GetPlayerSave`
  (returns (PlayerSave :type "/Game/MyBP/Structs/S_SaveData Structure"))
  (return (make `/Game/MyBP/Structs/S_SaveData` "0001.01.01-00.00.00")))

(fn `InitialiseSaveData`
  ;[0.4688 0.3558 0.1758] Fetches saved data if valid and sets this classes variables to our saved data
  (bind _savegamedata (message `/Game/MyBP/Interfaces/BPI_SaveGame.GetGameData` (`self.My Game Instance`)))
  (`/Engine/EditorBlueprintResources/StandardMacros.IsValid` _savegamedata
    (:`Is Valid`
      (`self.UsePlayerSave` (`/Game/MyBP/SaveGame/BP_SaveGame.S_SaveGameData` _savegamedata)))))

(fn `UsePlayerSave`
  (params (PlayerSave :type "/Game/MyBP/Structs/S_SaveData Structure")))

(fn `UserConstructionScript`)