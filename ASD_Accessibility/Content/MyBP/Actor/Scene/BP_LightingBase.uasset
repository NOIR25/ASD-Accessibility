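; BP_LightingBase is a scene lighting actor that changes its OutsideRect rect light to suit the current mood.
; On BeginPlay it caches the game mode and binds to its OnMoodChanged dispatcher.
; MoodChanged switches on the four moods and looks up each one's settings struct in a map.
; SetOutsideRect stores that struct and applies its colour, intensity, shape, barn door and temperature settings to the light.
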(event `self.ReceiveBeginPlay`
  (`self.FetchClasses`)
  (`self.BindToDispatchers`))

(event `MoodChanged`
  (params (Mood :type "/Game/MyBP/Enums/E_Moods Enum" :default "NewEnumerator0"))
  ;[0.1406 0.1059 0.07375] Switch, on selected mood
  (switch `/Game/MyBP/Enums/E_Moods` Mood
    (:`NewEnumerator0`
      ;[0.1406 0.1059 0.07375] using map to assign colour data unique to each mood
      (`self.SetOutsideRect` (`BlueprintMapLibrary.Map_Find` (`self.S_MoodLightArray0`) "NewEnumerator0")))
    (:`NewEnumerator5`
      (`self.SetOutsideRect` (`BlueprintMapLibrary.Map_Find` (`self.S_MoodLightArray0`) "NewEnumerator5")))
    (:`NewEnumerator1`
      (`self.SetOutsideRect` (`BlueprintMapLibrary.Map_Find` (`self.S_MoodLightArray0`) "NewEnumerator1")))
    (:`NewEnumerator2`
      (`self.SetOutsideRect` (`BlueprintMapLibrary.Map_Find` (`self.S_MoodLightArray0`) "NewEnumerator2")))))

(fn `BindToDispatchers`
  (add `/Game/MyBP/Actor/Player/BP_MyGM.OnMoodChanged` (`self.My Gamemode`) (`|CreateDelegate` :!event `MoodChanged`)))

(fn `FetchClasses`
  (bind _mygamemode (`/Game/MyBP/BFL/BFL_ClassFetcher.GetGM`))
  (set `self.My Gamemode` _mygamemode))

(fn `SetOutsideRect`
  (params (LightSettings :type "/Game/MyBP/Structs/S_RectLight Structure"))
  (bind _outsiderect (`self.OutsideRect`))
  (bind (_s_rectlightsettings_lightcolour _s_rectlightsettings_intensity _s_rectlightsettings_attenuationradius _s_rectlightsettings_sourcewidth _s_rectlightsettings_sourceheight _s_rectlightsettings_bardoorangle _s_rectlightsettings_barndoorlength _s_rectlightsettings_usetemperature _s_rectlightsettings_temperature) (break `/Game/MyBP/Structs/S_RectLight` (`self.S_RectLightSettings`)))
  (set `self.S_RectLightSettings` LightSettings)
  (`LightComponent.SetLightColor` _outsiderect _s_rectlightsettings_lightcolour true)
  (`LightComponent.SetIntensity` _outsiderect _s_rectlightsettings_intensity)
  (`LocalLightComponent.SetAttenuationRadius` _outsiderect _s_rectlightsettings_attenuationradius)
  (`RectLightComponent.SetSourceWidth` _outsiderect _s_rectlightsettings_sourcewidth)
  (`RectLightComponent.SetSourceHeight` _outsiderect _s_rectlightsettings_sourceheight)
  (`RectLightComponent.SetBarnDoorAngle` _outsiderect _s_rectlightsettings_bardoorangle)
  (`RectLightComponent.SetBarnDoorLength` _outsiderect _s_rectlightsettings_barndoorlength)
  (`LightComponent.SetUseTemperature` _outsiderect _s_rectlightsettings_usetemperature)
  (`LightComponent.SetTemperature` _outsiderect _s_rectlightsettings_temperature))

(fn `UserConstructionScript`)