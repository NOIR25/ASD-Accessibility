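; BP_SoundManager is a scene actor that reacts to mood changes in the game, apparently as the hook for mood-based sound.
; On BeginPlay it caches the game mode and binds to its OnMoodChanged dispatcher.
; The MoodChanged event switches on Calm, Focus, Over-Stimulated or Restless and calls a matching Cycle function.
; All four Cycle functions are empty stubs, so no audio logic exists yet.
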(event `self.ReceiveBeginPlay`
  (`self.Fetch Classes`)
  (`self.BindToDispatchers`))

(event `MoodChanged`
  (params (Mood :type "/Game/MyBP/Enums/E_Moods Enum" :default "NewEnumerator0"))
  (switch `/Game/MyBP/Enums/E_Moods` Mood
    (:`NewEnumerator0`
      (`self.CycleCalm`))
    (:`NewEnumerator5`
      (`self.CycleFocused`))
    (:`NewEnumerator1`
      (`self.CycleOverStimulated`))
    (:`NewEnumerator2`
      (`self.CycleRestless`))))

(fn `BindToDispatchers`
  (add `/Game/MyBP/Actor/Player/BP_MyGM.OnMoodChanged` (`self.My Gamemode`) (`|CreateDelegate` :!event `MoodChanged`)))

(fn `CycleCalm`)

(fn `CycleFocused`)

(fn `CycleOverStimulated`)

(fn `CycleRestless`)

(fn `Fetch Classes`
  (bind _mygamemode (`/Game/MyBP/BFL/BFL_ClassFetcher.GetGM`))
  (set `self.My Gamemode` _mygamemode))

(fn `UserConstructionScript`)