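; BP_MyDeck is a card deck actor for four categories: Lighting, Sound, Furniture and Decor.
; On BeginPlay it spawns one BP_Card per deck slot, each with a random row from that category's DataTable.
; DealCard reads the card's type and replaces that category's in-hand card, or toggles the selected card's flip if the held one is flipped.
; Flip events update card state and use a timeline to roll the mesh 180 degrees.
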(event `self.ReceiveBeginPlay`
  ;[0.09375 0.06431 0.01836] Spawn Initial Deck Cards And Assign A Randow Row From Their Respective Data Tables
  (bind _datatablerowhandle (`self.RandomDataTableRow` "/Game/MyBP/DT/DT_CardType_Lighting.DT_CardType_Lighting"))
  (`self.SpawnCardToDeck` (`self.UndealtLightingSlot`) (0.0 0.0 0.0) _datatablerowhandle)
  (bind _datatablerowhandle_2 (`self.RandomDataTableRow` "/Game/MyBP/DT/DT_CardType_Sound.DT_CardType_Sound"))
  (`self.SpawnCardToDeck` (`self.UndealtSoundSlot`) (0.0 0.0 0.0) _datatablerowhandle_2)
  (bind _datatablerowhandle_3 (`self.RandomDataTableRow` "/Game/MyBP/DT/DT_CardType_Furniture.DT_CardType_Furniture"))
  (`self.SpawnCardToDeck` (`self.UndealtFurnitureSlot`) (0.0 0.0 0.0) _datatablerowhandle_3)
  (bind _datatablerowhandle_4 (`self.RandomDataTableRow` "/Game/MyBP/DT/DT_CardType_Decor.DT_CardType_Decor"))
  (`self.SpawnCardToDeck` (`self.UndealtDecorSlot`) (0.0 0.0 0.0) _datatablerowhandle_4))

(event `/Game/MyBP/Interfaces/BPI_DeckFunctions.DealCard`
  (params (CardData :type "DataTableRowHandle Structure") (Card :type "/Game/MyBP/Actor/Cards/BP_Card Object Reference"))
  (set `self.SelectedCard` Card)
  (set `self.Card Data` CardData)
  (switch `/Game/MyBP/Enums/E_CardType` (`self.Get Spawned Card Type`)
    (:`NewEnumerator0`
      (bind _lightingcard (`self.LightingCard`)
        (:`then`
          (switch `/Game/MyBP/Enums/E_CardState` (`/Game/MyBP/Actor/Cards/BP_Card.CardState` _lightingcard)
            (:`NewEnumerator0`
              (bind _returnvalue (`self.SpawnCardToHand` (`self.InHandLightingSlot`) (0.0 0.0 0.0) _lightingcard :!label _label))
              (bind _output_get (set `self.LightingCard` _returnvalue))
              (set `/Game/MyBP/Actor/Cards/BP_Card.CardState` "NewEnumerator7" _output_get))
            (:`NewEnumerator7`
              (goto _label))
            (:`NewEnumerator8`
              (`self.FlipDeckCards`))))
        (:`else`
          (goto _label))))
    (:`NewEnumerator5`
      (bind _soundcard (`self.SoundCard`)
        (:`then`
          (switch `/Game/MyBP/Enums/E_CardState` (`/Game/MyBP/Actor/Cards/BP_Card.CardState` _soundcard)
            (:`NewEnumerator0`
              (bind _returnvalue_2 (`self.SpawnCardToHand` (`self.InHandSoundSlot`) (0.0 0.0 0.0) _soundcard :!label _label_2))
              (bind _output_get_2 (set `self.SoundCard` _returnvalue_2))
              (set `/Game/MyBP/Actor/Cards/BP_Card.CardState` "NewEnumerator7" _output_get_2))
            (:`NewEnumerator7`
              (goto _label_2))
            (:`NewEnumerator8`
              (`self.FlipDeckCards`))))
        (:`else`
          (goto _label_2))))
    (:`NewEnumerator2`
      (bind _furniturecard (`self.FurnitureCard`)
        (:`then`
          (switch `/Game/MyBP/Enums/E_CardState` (`/Game/MyBP/Actor/Cards/BP_Card.CardState` _furniturecard)
            (:`NewEnumerator0`
              (bind _returnvalue_3 (`self.SpawnCardToHand` (`self.InHandFurnitureSlot`) (0.0 0.0 0.0) _furniturecard :!label _label_3))
              (bind _output_get_3 (set `self.FurnitureCard` _returnvalue_3))
              (set `/Game/MyBP/Actor/Cards/BP_Card.CardState` "NewEnumerator7" _output_get_3))
            (:`NewEnumerator7`
              (goto _label_3))
            (:`NewEnumerator8`
              (`self.FlipDeckCards`))))
        (:`else`
          (goto _label_3))))
    (:`NewEnumerator1`
      (bind _decorcard (`self.DecorCard`)
        (:`then`
          (switch `/Game/MyBP/Enums/E_CardState` (`/Game/MyBP/Actor/Cards/BP_Card.CardState` _decorcard)
            (:`NewEnumerator0`
              (bind _returnvalue_4 (`self.SpawnCardToHand` (`self.InHandDecorSlot`) (0.0 0.0 0.0) _decorcard :!label _label_4))
              (bind _output_get_4 (set `self.DecorCard` _returnvalue_4))
              (set `/Game/MyBP/Actor/Cards/BP_Card.CardState` "NewEnumerator7" _output_get_4))
            (:`NewEnumerator7`
              (goto _label_4))
            (:`NewEnumerator8`
              (`self.FlipDeckCards`))))
        (:`else`
          (goto _label_4))))))

(event `/Game/MyBP/Interfaces/BPI_DeckFunctions.FlipCard`
  (params (Card :type "/Game/MyBP/Actor/Cards/BP_Card Object Reference"))
  (set `/Game/MyBP/Actor/Cards/BP_Card.isFlipped` true Card)
  (switch `/Game/MyBP/Enums/E_CardState` (`/Game/MyBP/Actor/Cards/BP_Card.CardState` Card)
    (:`NewEnumerator0`
      (`self.CE_FlipCard` Card))
    (:`NewEnumerator7`
      (set `/Game/MyBP/Actor/Cards/BP_Card.CardState` "NewEnumerator8" Card)
      (`self.CE_FlipCard` Card))))

(event `CE_FlipCard`
  (params (Card :type "/Game/MyBP/Actor/Cards/BP_Card Object Reference"))
  (bind _card (`/Game/MyBP/Actor/Cards/BP_Card.Card` Card))
  (bind (_relativerotation_roll _relativerotation_pitch _relativerotation_yaw) (`KismetMathLibrary.BreakRotator` (`SceneComponent.RelativeRotation` _card)))
  (`/Engine/EditorBlueprintResources/StandardMacros.IsValid` Card
    (:`Is Valid`
      (if (`/Game/MyBP/Actor/Cards/BP_Card.isFlipped` Card)
        (bind (_direction _alpha) (`Timeline|Lerp` :!via `PlayFromStart` :!label _label_5)
          (:`Update`
            (`SceneComponent.K2_SetRelativeRotation` _card (`KismetMathLibrary.MakeRotator` (`KismetMathLibrary.Lerp` 0.0 180.0 _alpha) _relativerotation_pitch _relativerotation_yaw) false false)))
        (else
          (goto _label_5 :!via `ReverseFromEnd`))))))

(event `/Game/MyBP/Interfaces/BPI_DeckFunctions.UnFlipCard`
  (params (Card :type "/Game/MyBP/Actor/Cards/BP_Card Object Reference"))
  (set `/Game/MyBP/Actor/Cards/BP_Card.isFlipped` false Card)
  (switch `/Game/MyBP/Enums/E_CardState` (`/Game/MyBP/Actor/Cards/BP_Card.CardState` Card)
    (:`NewEnumerator0`
      (`self.CE_FlipCard` Card))
    (:`NewEnumerator8`
      (set `/Game/MyBP/Actor/Cards/BP_Card.CardState` "NewEnumerator7" Card)
      (`self.CE_FlipCard` Card))))

(fn `FlipDeckCards`
  (if (`/Game/MyBP/Actor/Cards/BP_Card.isFlipped` (`self.SelectedCard`))
    (`self.UnFlipCard` (`self.SelectedCard`))
    (else
      (`self.FlipCard` (`self.SelectedCard`)))))

(fn `Get Spawned Card Type`
  (returns (Type :type "/Game/MyBP/Enums/E_CardType Enum"))
  (bind (_card_data_datatable _card_data_rowname) (break `DataTableRowHandle` (`self.Card Data`)))
  (bind _returnvalue (`|GetDataTableRow` _card_data_datatable _card_data_rowname)
    (:`then`
      (return (`.Type_22_7CFC8B4E4DDFFDA889CF7391A8D934E2` (break `/Game/MyBP/Structs/S_CardType` _returnvalue))))))

(fn `RandomDataTableRow`
  (params (Table :type "DataTable Object Reference"))
  (returns (DataTableRowHandle :type "DataTableRowHandle Structure"))
  (bind _outrownames (`DataTableFunctionLibrary.GetDataTableRowNames` Table))
  (return (make `DataTableRowHandle` Table (`KismetArrayLibrary.Array_Random` _outrownames))))

(fn `SpawnCardToDeck`
  (params (SpawnSlot :type "SceneComponent Object Reference") (SpawnOffset :type "Vector Structure") (CardData :type "DataTableRowHandle Structure"))
  (bind (_returnvalue_location _returnvalue_rotation _returnvalue_scale) (`KismetMathLibrary.BreakTransform` (`SceneComponent.K2_GetComponentToWorld` SpawnSlot)))
  (`|SpawnActorFromClass` "/Game/MyBP/Actor/Cards/BP_Card.BP_Card_C" (`KismetMathLibrary.MakeTransform` (+ _returnvalue_location SpawnOffset) _returnvalue_rotation _returnvalue_scale) "Undefined" "MultiplyWithRoot" null CardData self null))

(fn `SpawnCardToHand`
  (params (SpawnSlot :type "SceneComponent Object Reference") (SpawnOffset :type "Vector Structure") (Card :type "/Game/MyBP/Actor/Cards/BP_Card Object Reference"))
  (returns (ReturnValue :type "/Game/MyBP/Actor/Cards/BP_Card Object Reference"))
  (bind (_returnvalue_location _returnvalue_rotation _returnvalue_scale) (`KismetMathLibrary.BreakTransform` (`SceneComponent.K2_GetComponentToWorld` SpawnSlot)))
  (`/Engine/EditorBlueprintResources/StandardMacros.IsValid` Card
    (:`Is Valid`
      (`self.K2_DestroyActor` Card))
    (:`Is Not Valid`
      _))
  (bind _returnvalue (`|SpawnActorFromClass` "/Game/MyBP/Actor/Cards/BP_Card.BP_Card_C" (`KismetMathLibrary.MakeTransform` (+ _returnvalue_location SpawnOffset) _returnvalue_rotation _returnvalue_scale) "Undefined" "MultiplyWithRoot" null (`self.Card Data`) self null))
  (`KismetSystemLibrary.PrintString` "Dealt new card")
  (return _returnvalue))

(fn `UpdateCurrentDeck`
  (set `self.CurrentDeck` (`|MakeArray` (`self.LightingCard`) (`self.SoundCard`) (`self.FurnitureCard`) (`self.DecorCard`))))

(fn `UserConstructionScript`)