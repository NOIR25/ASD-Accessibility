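; BP_Card is a card actor whose data table row defines its type (lighting, soundscape, furniture or decor), primary rect light settings and colour palette.
; The construction script copies the light and palette data into variables; the type switch has empty branches.
; BeginPlay caches game mode and HUD references and creates a WB_Card widget.
; Taps message MyDeck to deal, flip or unflip the card according to CardState.
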(event `self.ReceiveBeginPlay`
  (`self.FetchClasses`)
  (`|CreateWidget` "/Game/MyBP/UI/WB_Card.WB_Card_C"))

(event `/Game/MyBP/Interfaces/BPI_Interactions.Tap Interact`
  (params (Interactor :type "Actor Object Reference"))
  (switch `/Game/MyBP/Enums/E_CardState` (`self.CardState`)
    (:`NewEnumerator0`
      (message `/Game/MyBP/Interfaces/BPI_DeckFunctions.DealCard` (`self.MyDeck`) (`self.DT`) self))
    (:`NewEnumerator7`
      (message `/Game/MyBP/Interfaces/BPI_DeckFunctions.FlipCard` (`self.MyDeck`) self))
    (:`NewEnumerator8`
      (message `/Game/MyBP/Interfaces/BPI_DeckFunctions.UnFlipCard` (`self.MyDeck`) self))))

(fn `FetchClasses`
  (bind _mygamemode (`/Game/MyBP/BFL/BFL_ClassFetcher.GetGM`))
  (set `self.My Gamemode` _mygamemode)
  (bind _hud (`/Game/MyBP/BFL/BFL_ClassFetcher.GetHUD`))
  (set `self.HUD` _hud))

(fn `SetCardData`
  (bind (_dt_datatable _dt_rowname) (break `DataTableRowHandle` (`self.DT`)))
  (bind _returnvalue (`|GetDataTableRow` _dt_datatable _dt_rowname)
    (:`then`
      (bind (_type _primaryrectlight _colourpallete) (break `/Game/MyBP/Structs/S_CardType` _returnvalue))
      (switch `/Game/MyBP/Enums/E_CardType` _type
        (:`NewEnumerator0`
          _)
        (:`NewEnumerator5`
          _)
        (:`NewEnumerator2`
          _)
        (:`NewEnumerator1`
          _))
      (bind (_lightcolour _intensity _attenuationradius _sourcewidth _sourceheight _bardoorangle _barndoorlength _usetemperature _temperature) (break `/Game/MyBP/Structs/S_RectLight` _primaryrectlight))
      (set `self.PrimaryRectLight` (make `/Game/MyBP/Structs/S_RectLight` _lightcolour _intensity _attenuationradius _sourcewidth _sourceheight _bardoorangle _barndoorlength _usetemperature _temperature))
      (bind (_colour0 _colour1 _colour2 _colour3 _colour4 _colour5) (break `/Game/MyBP/Structs/S_ColourPallete1` _colourpallete))
      (set `self.ColourPallete` (make `/Game/MyBP/Structs/S_ColourPallete1` _colour0 _colour1 _colour2 _colour3 _colour4 _colour5)))))

(fn `UserConstructionScript`
  (`self.SetCardData`))